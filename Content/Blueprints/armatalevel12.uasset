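; Cannon actor (armata) for level 12 that repeatedly spawns Pocisk projectiles from two arrow components.
; Tick drives both branches through latent Delays, which act as fire timers because retriggers are ignored while counting down.
; Arrow fires after Opoznienie, while Arrow2 waits an extra Opoznienie2 first, giving it a longer cycle.
; Both branches feed a shared SetLifeSpan call driven by Dlugoscistnienia.
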(event EventTick
  (params (DeltaSeconds :type Float%20%28single-precision%29))
  (Utilities|FlowControl|Sequence
    (:then_0
      (Utilities|FlowControl|Delay (Variables|Default|GetOpoznienie2))
      (Utilities|FlowControl|Delay (Variables|Default|GetOpoznienie))
      (Game|SpawnActorfromClass "/Game/Blueprints/pocisk.pocisk_C" (Transformation|GetWorldTransform (Variables|Default|GetArrow2)) "Undefined" 0 0))
    (:then_1
      (Utilities|FlowControl|Delay (Variables|Default|GetOpoznienie))
      (Game|SpawnActorfromClass "/Game/Blueprints/pocisk.pocisk_C" (Transformation|GetWorldTransform (Variables|Default|GetArrow)) "Undefined" 0 0)))
  (Actor|SetLifeSpan (Variables|Default|Getdlugoscistnienia)))

(fn ConstructionScript)